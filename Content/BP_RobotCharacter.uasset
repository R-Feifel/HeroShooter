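; BP_RobotCharacter is a robot character Blueprint with a first-person mesh, a shadow body mesh and a weapon mesh for each.
; On BeginPlay it attaches the player weapon to the first-person GripPoint socket and the shadow weapon to the shadow mesh's middle_01_r socket.
; Each weapon snaps to its socket's world transform, then receives a hard-coded world-space offset to correct alignment.
; It contains no other active logic.
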(event EventBeginPlay
  (bind _shadowweaponmesh (Variables|Default|GetShadowWeaponMesh))
  (bind _playerweaponmesh (Variables|Default|GetPlayerWeaponMesh))
  (bind _shadowplayermesh (Variables|Default|GetShadowPlayerMesh))
  (bind _playermesh1p (Variables|Default|GetPlayerMesh1P))
  (bind _returnvalue (Transformation|GetSocketTransform _playermesh1p "GripPoint" "RTS_World"))
  (bind _returnvalue_2 (Transformation|GetSocketTransform _shadowplayermesh "middle_01_r" "RTS_World"))
  ;[0 0 0] Nonsense required to align Player Weapon Mesh with Player Mesh
  (Transformation|AttachComponentToComponent _playerweaponmesh _playermesh1p "GripPoint" "KeepRelative" "KeepRelative" "KeepRelative" true)
  (Transformation|SetWorldLocationAndRotation _playerweaponmesh (.location _returnvalue) (.rotation _returnvalue) false true)
  (Class|SceneComponent|AddWorldTransform _playerweaponmesh (Math|Transform|MakeTransform "0.000000,-0.000000,-2.500000" "-6.000000,-3.000000, 0" "1.000000,1.000000,1.000000") false true)
  ;[0 0 0] Nonsense required to align Shadow Weapon Mesh with Shadow Player Mesh
  (Transformation|AttachComponentToComponent _shadowweaponmesh _shadowplayermesh "middle_01_r" "KeepRelative" "KeepRelative" "KeepRelative" true)
  (Transformation|SetWorldLocationAndRotation _shadowweaponmesh (.location _returnvalue_2) (.rotation _returnvalue_2) false true)
  (Class|SceneComponent|AddWorldTransform _shadowweaponmesh (Math|Transform|MakeTransform "-5.000000,-5.000000,0.000000" "17.000000,160.000000, 0" "1.000000,1.000000,1.000000") false true))

(event Collision|EventActorBeginOverlap
  (params (OtherActor :type Actor%20Object%20Reference)))

(event EventTick
  (params (DeltaSeconds :type Float%20%28single-precision%29)))

(fn ConstructionScript)